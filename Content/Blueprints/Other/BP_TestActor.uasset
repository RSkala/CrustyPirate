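; BP_TestActor is a test actor that exercises native C++ functions exposed to Blueprint as implementable events, native events and pure functions.
; On BeginPlay it calls each of the three event variants, and their Blueprint overrides print marker strings to the log.
; The native event override also calls its parent implementation, then prints the int, bool and string outputs of a pure function.
; The returning override outputs zero.
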(event `self.ReceiveBeginPlay`
  (`self.BlueprintImplementableEventFunction`)
  (`self.BlueprintNativeEventFunction`)
  (`self.BlueprintNativeEventWithReturnFunction`))

(event `self.ReceiveTick`
  (params (DeltaSeconds :type "Float (single-precision)")))

(event `self.BlueprintNativeEventFunction`
  (bind (_outtestint _outtestbool _outteststring) (`self.BlueprintPureFunction2`))
  (`KismetSystemLibrary.PrintString` "blueprint native event bp" false)
  (`parent.BlueprintNativeEventFunction`)
  (`KismetSystemLibrary.PrintString` (`KismetStringLibrary.Conv_IntToString` _outtestint))
  (`KismetSystemLibrary.PrintString` (`KismetStringLibrary.Conv_BoolToString` _outtestbool))
  (`KismetSystemLibrary.PrintString` _outteststring))

(event `self.BlueprintImplementableEventFunction`
  (`KismetSystemLibrary.PrintString` "blueprint implementable event bp" false))

(fn `BlueprintNativeEventWithReturnFunction`
  (returns (ReturnValue :type Integer))
  (`KismetSystemLibrary.PrintString` "native event with return bp" false)
  (return 0))

(fn `NewFunction`)

(fn `UserConstructionScript`)